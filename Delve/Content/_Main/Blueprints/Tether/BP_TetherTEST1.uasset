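; BP_TetherTEST1 is a test tether actor that stretches between the world origin and player character 0.
; Each Tick it moves to the midpoint, aligns its Z axis along that line with MakeRotFromZX, and scales Z to the distance divided by 100.
; It prints that scale factor every frame for debugging.
; The Start location saved on BeginPlay is never read, as the origin is hard-coded.
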(event `self.ReceiveBeginPlay`
  (set `self.Start` (`self.K2_GetActorLocation`)))

(event `self.ReceiveTick`
  (params (DeltaSeconds :type "Float (single-precision)"))
  (bind _end (`self.End`))
  (bind _returnvalue (/ (`KismetMathLibrary.VSize` (- (0.0 0.0 0.0) (`self.End`))) 100.0))
  (set `self.End` (`self.K2_GetActorLocation` (`GameplayStatics.GetPlayerCharacter` 0)))
  (`self.K2_SetActorRotation` (`KismetMathLibrary.MakeRotFromZX` (`KismetMathLibrary.Normal` (- (0.0 0.0 0.0) _end)) _end))
  (`self.K2_SetActorLocation` (/ (+ (0.0 0.0 0.0) (`self.End`)) 2.0))
  (`KismetSystemLibrary.PrintString` (`KismetStringLibrary.Conv_DoubleToString` _returnvalue))
  (`self.SetActorScale3D` (`KismetMathLibrary.MakeVector` 1.0 1.0 _returnvalue)))

(fn `UserConstructionScript`)