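; BP_Shop is a shop pickup that offers one random item and grants its passive bonus, with no cost check.
; BeginPlay picks a random data table row, sets the item mesh and fills a description widget component added in the construction script.
; Sphere overlap by a BPI_IPlayer actor enables input and shows the item text and widget.
; Pressing E sends the bonus through the interface, hides the mesh and locks further use.
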(event `self.ReceiveBeginPlay`
  ;[1 1 1] Setting random item struct & mesh from the items data table
  (bind _outrownames (`DataTableFunctionLibrary.GetDataTableRowNames` (`self.Items`)))
  (bind _returnvalue (`|GetDataTableRow` "/Game/_Main/Blueprints/Shop/DT_Item.DT_Item" (`KismetArrayLibrary.Array_Random` _outrownames))
    (:`then`
      (bind _output_get (set `self.Bonus Struct` (make `/Game/_Main/Blueprints/Structs/Shop/S_Item` (break `/Game/_Main/Blueprints/Structs/Shop/S_Item` _returnvalue) (`.ItemType_21_57364E6A479769CBE3DE43B0D83A6CB9` (break `/Game/_Main/Blueprints/Structs/Shop/S_Item` _returnvalue)) (`.ItemMesh_13_B14460B84C32510E59321BAA07984EE5` (break `/Game/_Main/Blueprints/Structs/Shop/S_Item` _returnvalue)) (`.ItemDescription_28_BF4868524D45789C25FD8F9DF78C1B61` (break `/Game/_Main/Blueprints/Structs/Shop/S_Item` _returnvalue)) (`.Effect_31_551EF87D48059BF33615BF996FCF6E2C` (break `/Game/_Main/Blueprints/Structs/Shop/S_Item` _returnvalue)) (`.Rarity_18_8877A1654349700FAAC8CC995A528E01` (break `/Game/_Main/Blueprints/Structs/Shop/S_Item` _returnvalue)) (`.ItemBonus_27_746F015E4DBFB895408FFDB110AA06DF` (break `/Game/_Main/Blueprints/Structs/Shop/S_Item` _returnvalue)))))
      (`StaticMeshComponent.SetStaticMesh` (`self.Item`) (`.ItemMesh_13_B14460B84C32510E59321BAA07984EE5` (break `/Game/_Main/Blueprints/Structs/Shop/S_Item` _output_get)))
      (bind _asw_item_description (cast `/Game/_Main/Blueprints/Widgets/W_ItemDescription` (`WidgetComponent.GetWidget` (`self.WidgetConstruction`))))
      (bind _output_get_2 (set `self.Widget` _asw_item_description))
      (`/Game/_Main/Blueprints/Widgets/W_ItemDescription.Format Item Text` _output_get_2 (`self.Bonus Struct`)))))

(event `self.Sphere.OnComponentBeginOverlap`
  (params (OverlappedComponent :type "PrimitiveComponent Object Reference") (OtherActor :type "Actor Object Reference") (OtherComp :type "PrimitiveComponent Object Reference") (OtherBodyIndex :type Integer) (bFromSweep :type Boolean) (SweepResult :type "HitResult Structure (by ref)"))
  (bind _bonus_struct_itemname (break `/Game/_Main/Blueprints/Structs/Shop/S_Item` (`self.Bonus Struct`)))
  ;[1 1 1] Setting the ability to buy the item
  (if (`self.TookItem?`)
    _
    (elif (`KismetSystemLibrary.DoesImplementInterface` OtherActor "/Game/_Main/Blueprints/Interfaces/Player/BPI_IPlayer.BPI_IPlayer_C")
      (set `self.Player` OtherActor)
      (`self.EnableInput` (`GameplayStatics.GetPlayerController` 0))
      (message `/Game/_Main/Blueprints/Interfaces/Player/BPI_SetUIItemTextVisible.Set UI Item Text Visible` (`self.Player`) _bonus_struct_itemname)
      (`Widget.SetVisibility` (`self.Widget`) "Visible"))))

(event `self.Sphere.OnComponentEndOverlap`
  (params (OverlappedComponent :type "PrimitiveComponent Object Reference") (OtherActor :type "Actor Object Reference") (OtherComp :type "PrimitiveComponent Object Reference") (OtherBodyIndex :type Integer))
  ;[1 1 1] Setting the ability to buy the item
  (if (`self.TookItem?`)
    _
    (elif (`KismetSystemLibrary.DoesImplementInterface` OtherActor "/Game/_Main/Blueprints/Interfaces/Player/BPI_IPlayer.BPI_IPlayer_C")
      (`self.DisableInput` (`GameplayStatics.GetPlayerController` 0))
      (message `/Game/_Main/Blueprints/Interfaces/Player/BPI_SetUIItemTextInvisible.Set UI Item Text Invisible` (`self.Player`))
      (`Widget.SetVisibility` (`self.Widget`) "Hidden"))))

(event `Key|E`
  (params (Key :type "Key Structure"))
  (bind (_bonus_struct_itemname _bonus_struct_itemtype _bonus_struct_itemmesh _bonus_struct_itemdescription _bonus_struct_effect _bonus_struct_rarity _bonus_struct_itembonus) (break `/Game/_Main/Blueprints/Structs/Shop/S_Item` (`self.Bonus Struct`)))
  ;[1 1 1] Buy logic when pressing "[E]"
  (:`Pressed`
    (if (not (`self.TookItem?`))
      (message `/Game/_Main/Blueprints/Interfaces/Player/BPI_AddPassive.Add Passive` (`self.Player`) _bonus_struct_itembonus)
      (`SceneComponent.SetVisibility` (`self.Item`) false false)
      (set `self.TookItem?` true)
      (message `/Game/_Main/Blueprints/Interfaces/Player/BPI_SetUIItemTextInvisible.Set UI Item Text Invisible` (`self.Player`)))))

(fn `UserConstructionScript`
  (bind _returnvalue (`AddComponent|NODE_AddWidgetComponent-0`))
  (set `self.WidgetConstruction` _returnvalue))