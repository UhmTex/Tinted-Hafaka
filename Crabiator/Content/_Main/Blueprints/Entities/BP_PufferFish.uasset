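; BP_PufferFish is an entity that builds up aggro in steps and explodes on the fourth.
; AggroBuildup is gated by a flag that a delay re-arms after each of the first three steps.
; Explode acts only if the player overlaps the Hitbox, sending damage and pushback messages along the arrow's forward vector.
; It then spawns an explosion effect and a random number of fishbones, destroying itself within that spawn loop.
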(event `Aggro Buildup`
  (bind _builduprate (`self.BuildupRate`))
  (if (`self.bCanBuildupAggro`)
    (set `self.bCanBuildupAggro` false)
    (`/Engine/EditorBlueprintResources/StandardMacros.IncrementInt` (`self.Buildup`)
      (:`  `
        (`KismetSystemLibrary.PrintString` "build up")
        (if (== (`self.Buildup`) 4)
          (`KismetSystemLibrary.Delay` _builduprate)
          (`self.Explode`)
          (else
            (`KismetSystemLibrary.Delay` _builduprate)
            (set `self.bCanBuildupAggro` true)))))))

(event `Explode`
  (bind _returnvalue (`self.K2_GetActorLocation`))
  (bind _output (`|GetArrayItem` (`PrimitiveComponent.GetOverlappingActors` (`self.Hitbox`) "/Game/FirstPerson/Blueprints/BP_FirstPersonCharacter.BP_FirstPersonCharacter_C")))
  (`/Engine/EditorBlueprintResources/StandardMacros.IsValid` _output
    (:`Is Valid`
      (message `/Game/_Main/Blueprints/Interfaces/Entities/BPI_IEntity.Take Damage` _output (`.EntityDamage_13_B4048A624DED884F8D8799BF30947D11` (break `/Game/_Main/Blueprints/Structs/Entities/S_Entity` (`self.Entity Data`))))
      (message `/Game/_Main/Blueprints/Interfaces/Player/BPI_IPlayer.Pushback` _output (`SceneComponent.GetForwardVector` (`self.Arrow1`)) (`self.Pushback Force`))
      (`GameplayStatics.SpawnEmitterAtLocation` "/Game/StarterContent/Particles/P_Explosion.P_Explosion" _returnvalue (struct) (2.0 2.0 2.0))
      (for _ (range (+ (`KismetMathLibrary.RandomInteger` 5) 1))
        (`|SpawnActorFromClass` "/Game/_Main/Blueprints/Fishbones/BP_Fishbone.BP_Fishbone_C" (`KismetMathLibrary.MakeTransform` _returnvalue) "AlwaysSpawn" "MultiplyWithRoot" null null)
        (`self.K2_DestroyActor`)))))

(fn `UserConstructionScript`
  (`parent.UserConstructionScript`))