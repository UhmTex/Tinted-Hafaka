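; BP_Spawn is a spawner that populates a circular arena with pufferfish and baby squid.
; A looping timer started at BeginPlay drives spawning, with each spawn picking one of the two classes at random.
; Positions are uniformly distributed over a disc around the actor using square-root radius sampling, sized by the Arena component's bounds and raised slightly above it.
; Spawns adjust to avoid collisions or are skipped.
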(event `self.ReceiveBeginPlay`
  (`KismetSystemLibrary.K2_SetTimerDelegate` (`|CreateDelegate` :!event `Spawn Entity`) 3.0 true))

(event `Spawn Entity`
  (bind (_returnvalue_x _returnvalue_y) (`KismetMathLibrary.BreakVector` (`self.K2_GetActorLocation`)))
  (bind _returnvalue_x_2 (`KismetMathLibrary.BreakVector` (`self.K2_GetActorLocation`)))
  (set `self.R` (* (.x (`.BoxExtent` (`KismetSystemLibrary.GetComponentBounds` (`self.Arena`)))) (`KismetMathLibrary.Sqrt` (`KismetMathLibrary.RandomFloat`))))
  (set `self.Theta` (* (* (`KismetMathLibrary.RandomFloat`) 2.0) (`KismetMathLibrary.GetPI`)))
  (set `self.Spawn X` (+ _returnvalue_x_2 (* (`self.R`) (`KismetMathLibrary.Cos` (`self.Theta`)))))
  (set `self.Spawn Y` (+ _returnvalue_y (* (`self.R`) (`KismetMathLibrary.Sin` (`self.Theta`)))))
  (set `self.Spawn Z` (+ (.z (`SceneComponent.K2_GetComponentLocation` (`self.Arena`))) 30.0))
  (switch `int` (`KismetMathLibrary.RandomIntegerInRange` 0 1)
    (:`0`
      (`|SpawnActorFromClass` "/Game/_Main/Blueprints/Entities/Entities/PufferFish/BP_PufferFish.BP_PufferFish_C" (`KismetMathLibrary.MakeTransform` (`KismetMathLibrary.MakeVector` (`self.Spawn X`) (`self.Spawn Y`) (`self.Spawn Z`))) "AdjustIfPossibleButDontSpawnIfColliding" "MultiplyWithRoot" null null))
    (:`1`
      (`|SpawnActorFromClass` "/Game/_Main/Blueprints/Entities/Entities/BabySquid/BP_BabySquid.BP_BabySquid_C" (`KismetMathLibrary.MakeTransform` (`KismetMathLibrary.MakeVector` (`self.Spawn X`) (`self.Spawn Y`) (`self.Spawn Z`))) "AdjustIfPossibleButDontSpawnIfColliding" "MultiplyWithRoot" null null))))

(fn `UserConstructionScript`)