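; BP_BabySquid is a squid entity that fires ink projectiles and feeds player proximity to its AI.
; FireInk spawns a half-scale BP_InkProjectile at the Sphere component's transform, passing EntityData damage and launching it along the actor's forward vector.
; SpookZone overlaps with BPI_IPlayer actors drive the RunAway blackboard key: false on entering, true on leaving.
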(event `Fire Ink`
  (bind (_entity_data_entityname _entity_data_entitytitle _entity_data_entityhp _entity_data_entityability _entity_data_entitydamage) (break `/Game/_Main/Blueprints/Structs/Entities/S_Entity` (`self.Entity Data`)))
  (bind (_returnvalue_location _returnvalue_rotation) (`KismetMathLibrary.BreakTransform` (`SceneComponent.K2_GetComponentToWorld` (`self.Sphere`))))
  (bind _returnvalue (`|SpawnActorFromClass` "/Game/_Main/Blueprints/Entities/Entities/BabySquid/BP_InkProjectile.BP_InkProjectile_C" (`KismetMathLibrary.MakeTransform` _returnvalue_location _returnvalue_rotation (0.5 0.5 0.5)) "Undefined" "MultiplyWithRoot" null null))
  (set `/Game/_Main/Blueprints/Entities/Entities/BabySquid/BP_InkProjectile.Damage` _entity_data_entitydamage _returnvalue)
  (set `MovementComponent.Velocity` (* (`KismetMathLibrary.GetForwardVector` (`self.K2_GetActorRotation` self)) 3000.0) (`/Game/_Main/Blueprints/Entities/Entities/BabySquid/BP_InkProjectile.ProjectileMovement` _returnvalue)))

(event `self.SpookZone.OnComponentBeginOverlap`
  (params (OverlappedComponent :type "PrimitiveComponent Object Reference") (OtherActor :type "Actor Object Reference") (OtherComp :type "PrimitiveComponent Object Reference") (OtherBodyIndex :type Integer) (bFromSweep :type Boolean) (SweepResult :type "HitResult Structure (by ref)"))
  (if (`KismetSystemLibrary.DoesImplementInterface` OtherActor "/Game/_Main/Blueprints/Interfaces/Player/BPI_IPlayer.BPI_IPlayer_C")
    (`BlackboardComponent.SetValueAsBool` (`AIBlueprintHelperLibrary.GetBlackboard` null) "RunAway" false)))

(event `self.SpookZone.OnComponentEndOverlap`
  (params (OverlappedComponent :type "PrimitiveComponent Object Reference") (OtherActor :type "Actor Object Reference") (OtherComp :type "PrimitiveComponent Object Reference") (OtherBodyIndex :type Integer))
  (bind _returnvalue (`AIBlueprintHelperLibrary.GetBlackboard` null))
  (if (`KismetSystemLibrary.DoesImplementInterface` OtherActor "/Game/_Main/Blueprints/Interfaces/Player/BPI_IPlayer.BPI_IPlayer_C")
    (`/Engine/EditorBlueprintResources/StandardMacros.IsValid` _returnvalue
      (:`Is Valid`
        (`BlackboardComponent.SetValueAsBool` _returnvalue "RunAway" true)))))

(fn `UserConstructionScript`
  (`parent.UserConstructionScript`))