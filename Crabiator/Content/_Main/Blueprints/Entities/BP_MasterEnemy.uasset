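; BP_MasterEnemy is an enemy Blueprint, apparently a base class by its name, that handles damage and death.
; TakeDamage subtracts damage from HP in the EntityData struct and calls Death at zero or below.
; Death plays a Niagara effect, then runs a random-length loop spawning BP_Fishbone actors at the enemy's location.
; The kill notification to BP_FirstPersonCharacter and DestroyActor both sit inside that loop body, rather than after it.
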(event `/Game/_Main/Blueprints/Interfaces/Entities/BPI_IEntity.Take Damage`
  (params (Damage :type "Float (double-precision)"))
  (bind (_entity_data_entityname _entity_data_entitytitle _entity_data_entityhp) (break `/Game/_Main/Blueprints/Structs/Entities/S_Entity` (`self.Entity Data`)))
  (bind _structout (setmembers `/Game/_Main/Blueprints/Structs/Entities/S_Entity` :`StructRef` (`self.Entity Data`) :`Entity HP` (- _entity_data_entityhp Damage)))
  (if (<= (`.EntityHP_10_85FFC4AC46E62A3DB812EA88D00E176D` (break `/Game/_Main/Blueprints/Structs/Entities/S_Entity` _structout)) 0.0)
    (`self.Death`)))

(event `Death`
  (`NiagaraFunctionLibrary.SpawnSystemAtLocation` "/Game/_Main/VFX/NS_EnemiesDeath/NS_EnemiesDeath.NS_EnemiesDeath" (`self.K2_GetActorLocation`))
  (for _ (range (+ (`KismetMathLibrary.RandomInteger` 5) 1))
    (`|SpawnActorFromClass` "/Game/_Main/Blueprints/Fishbones/BP_Fishbone.BP_Fishbone_C" (`KismetMathLibrary.MakeTransform` (`self.K2_GetActorLocation`)) "AlwaysSpawn" "MultiplyWithRoot" null null)
    (bind _asbp_first_person_character (cast `/Game/FirstPerson/Blueprints/BP_FirstPersonCharacter` (`GameplayStatics.GetPlayerCharacter` 0)))
    (`/Game/FirstPerson/Blueprints/BP_FirstPersonCharacter.Enemy killed` _asbp_first_person_character)
    (`self.K2_DestroyActor`)))

(fn `UserConstructionScript`)