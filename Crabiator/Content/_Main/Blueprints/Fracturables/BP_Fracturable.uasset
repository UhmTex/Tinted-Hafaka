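; BP_Fracturable is a breakable Chaos geometry collection actor that fractures at a given hit point.
; Its Break event spawns a scaled-down FS_MasterField just behind the impact surface along the hit normal, configures it as a short-lived radial impulse and triggers it.
; The IsBroken flag and the per-particle collision disabling are present but disconnected, so neither runs.
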(event `/Game/_Main/Blueprints/Interfaces/Chaos/BPI_Fracturable.Break`
  (params (`Hit Result` :type "HitResult Structure"))
  (bind _output_get (set `self.Hit Result` `Hit Result`))
  (bind (_returnvalue_location _returnvalue_rotation) (`KismetMathLibrary.BreakTransform` (`KismetMathLibrary.Conv_VectorToTransform` (`.ImpactPoint` (`GameplayStatics.BreakHitResult` _output_get)))))
  (bind _returnvalue (`|SpawnActorFromClass` "/Engine/EditorResources/FieldNodes/FS_MasterField.FS_MasterField_C" (`KismetMathLibrary.MakeTransform` (+ _returnvalue_location (* (`.ImpactNormal` (`GameplayStatics.BreakHitResult` _output_get)) -3.0)) _returnvalue_rotation (0.7 0.7 0.7)) "Undefined" "MultiplyWithRoot" null null))
  (set `self.ChaosImpactFieldRef` _returnvalue)
  (set `/Engine/EditorResources/FieldNodes/FS_MasterField.ActivationType` "NewEnumerator4" (`self.ChaosImpactFieldRef`))
  (set `/Engine/EditorResources/FieldNodes/FS_MasterField.FieldLifespan` 0.1 (`self.ChaosImpactFieldRef`))
  (set `/Engine/EditorResources/FieldNodes/FS_MasterField.Radial Magnitude` 3000.0 (`self.ChaosImpactFieldRef`))
  (`/Engine/EditorResources/FieldNodes/FS_MasterField.CE_Trigger` (`self.ChaosImpactFieldRef`)))

(fn `UserConstructionScript`)