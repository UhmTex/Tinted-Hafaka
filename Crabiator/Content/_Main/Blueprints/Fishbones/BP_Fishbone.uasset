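; BP_Fishbone is a collectible pickup worth a random fishbone value.
; On spawn its physics Cube pops up with a randomized sideways force, becomes collectible after a short delay, then stops simulating physics.
; Sphere overlap with a BPI_IPlayer actor moves the Cube to the player, sends the value through CollectFishboneMessage and destroys the pickup.
; Early overlaps retry after a brief delay while that player remains the first overlapping character.
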(event `self.ReceiveBeginPlay`
  (set `self.Fishbone Value` (`KismetMathLibrary.RandomIntegerInRange` 5 30))
  (`PrimitiveComponent.AddForce` (`self.Cube`) (* (`KismetMathLibrary.MakeVector` (`KismetArrayLibrary.Array_Random` (`self.RandomTable`)) (`KismetArrayLibrary.Array_Random` (`self.RandomTable`)) 1.0) (35.0 35.0 50.0)) "None" false)
  (`KismetSystemLibrary.Delay` 1.0)
  (set `self.bCanPickUp` true)
  (`KismetSystemLibrary.Delay` 2.0)
  (`PrimitiveComponent.SetSimulatePhysics` (`self.Cube`) false))

(event `self.Sphere.OnComponentBeginOverlap`
  (params (OverlappedComponent :type "PrimitiveComponent Object Reference") (OtherActor :type "Actor Object Reference") (OtherComp :type "PrimitiveComponent Object Reference") (OtherBodyIndex :type Integer) (bFromSweep :type Boolean) (SweepResult :type "HitResult Structure (by ref)"))
  (bind _output (`|GetArrayItem` (`PrimitiveComponent.GetOverlappingActors` (`self.Sphere`) "/Game/FirstPerson/Blueprints/BP_FirstPersonCharacter.BP_FirstPersonCharacter_C")))
  (if (`KismetSystemLibrary.DoesImplementInterface` OtherActor "/Game/_Main/Blueprints/Interfaces/Player/BPI_IPlayer.BPI_IPlayer_C")
    (set `self.Player` OtherActor)
    (if (`KismetSystemLibrary.IsValid` (`self.Player`))
      (if (`self.bCanPickUp`) :!label _label
        (`KismetSystemLibrary.MoveComponentTo` (`self.Cube`) (`self.K2_GetActorLocation` (`self.Player`)))
        (message `/Game/_Main/Blueprints/Interfaces/Player/BPI_IPlayer.Collect Fishbone` (`self.Player`) (`self.Fishbone Value`))
        (`self.K2_DestroyActor`)
        (else
          (`KismetSystemLibrary.Delay` 0.2)
          (`/Engine/EditorBlueprintResources/StandardMacros.IsValid` _output
            (:`Is Valid`
              (if (== _output (`self.Player`))
                (goto _label)))))))))

(fn `UserConstructionScript`)