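; BP_LevelStarter is an interactable level transition actor that opens the Game_Main level when the player uses it.
; Its Trigger component enables input on the actor while an overlapping actor implementing BPI_IPlayer is inside, and disables it on exit.
; Pressing E rolls the Transitor2 component to a fixed angle, like a thrown switch, then loads the level after a short delay.
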(event `self.Trigger.OnComponentBeginOverlap`
  (params (OverlappedComponent :type "PrimitiveComponent Object Reference") (OtherActor :type "Actor Object Reference") (OtherComp :type "PrimitiveComponent Object Reference") (OtherBodyIndex :type Integer) (bFromSweep :type Boolean) (SweepResult :type "HitResult Structure (by ref)"))
  (if (`KismetSystemLibrary.DoesImplementInterface` OtherActor "/Game/_Main/Blueprints/Interfaces/Player/BPI_IPlayer.BPI_IPlayer_C")
    (`self.EnableInput` (`GameplayStatics.GetPlayerController` 0))))

(event `self.Trigger.OnComponentEndOverlap`
  (params (OverlappedComponent :type "PrimitiveComponent Object Reference") (OtherActor :type "Actor Object Reference") (OtherComp :type "PrimitiveComponent Object Reference") (OtherBodyIndex :type Integer))
  (if (`KismetSystemLibrary.DoesImplementInterface` OtherActor "/Game/_Main/Blueprints/Interfaces/Player/BPI_IPlayer.BPI_IPlayer_C")
    (`self.DisableInput` (`GameplayStatics.GetPlayerController` 0))))

(event `Key|E`
  (params (Key :type "Key Structure"))
  (bind _transitor2 (`self.Transitor2`))
  (bind (_relativerotation_roll _relativerotation_pitch _relativerotation_yaw) (`KismetMathLibrary.BreakRotator` (`SceneComponent.RelativeRotation` _transitor2)))
  (:`Pressed`
    (`SceneComponent.K2_SetRelativeRotation` _transitor2 (`KismetMathLibrary.MakeRotator` 30.0 _relativerotation_pitch _relativerotation_yaw) false false)
    (`KismetSystemLibrary.Delay` 1.0)
    (`GameplayStatics.OpenLevelBySoftObjectPtr` "/Game/_Main/Levels/Game_Main.Game_Main")))

(fn `UserConstructionScript`)